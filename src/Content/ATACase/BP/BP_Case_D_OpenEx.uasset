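; Interactive ATA case actor that the player opens and closes with the E key while inside its trigger box.
; Box overlap toggles the PressE prompt and opens or closes a gate; entering also enables input, which is never disabled.
; E presses enlarge the prompt until release and, through the gate, drive a FlipFlop alternating the skeletal mesh's extended-opening and closing animations.
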(event OnComponentBeginOverlap(Box)
  (params (OverlappedComponent :type Primitive%20Component%20Object%20Reference) (OtherActor :type Actor%20Object%20Reference) (OtherComp :type Primitive%20Component%20Object%20Reference) (OtherBodyIndex :type Integer) (bFromSweep :type Boolean) (SweepResult :type Hit%20Result%20Structure%20%28by%20ref%29))
  (bind _skeletalmesh (Variables|Default|GetSkeletalMesh))
  (Variables|Default|SetOverlap%20Trig true)
  (if (Variables|Default|GetOverlap%20Trig)
    (Rendering|ToggleVisibility (Variables|Default|GetPress%20E) false)
    (Input|EnableInput (Game|GetPlayerController 0))
    (Utilities|FlowControl|Gate true) ; enters at Open
    (else
      (Rendering|ToggleVisibility (Variables|Default|GetPress%20E) false)
      (Utilities|FlowControl|Gate true) ; enters at Close
    )))

(event OnComponentEndOverlap(Box)
  (params (OverlappedComponent :type Primitive%20Component%20Object%20Reference) (OtherActor :type Actor%20Object%20Reference) (OtherComp :type Primitive%20Component%20Object%20Reference) (OtherBodyIndex :type Integer))
  (bind _skeletalmesh (Variables|Default|GetSkeletalMesh))
  (Variables|Default|SetOverlap%20Trig false)
  (if (Variables|Default|GetOverlap%20Trig)
    (Rendering|ToggleVisibility (Variables|Default|GetPress%20E) false)
    (Input|EnableInput (Game|GetPlayerController 0))
    (Utilities|FlowControl|Gate true) ; enters at Open
    (else
      (Rendering|ToggleVisibility (Variables|Default|GetPress%20E) false)
      (Utilities|FlowControl|Gate true) ; enters at Close
    )))

(event EventBeginPlay)

(event Collision|EventActorBeginOverlap
  (params (OtherActor :type Actor%20Object%20Reference)))

(event EventTick
  (params (DeltaSeconds :type Float%20%28single-precision%29)))

(event Input|KeyboardEvents|E
  (params (Key :type Key%20Structure :default "AnyKey"))
  (bind _skeletalmesh (Variables|Default|GetSkeletalMesh))
  (bind _press_e (Variables|Default|GetPress%20E))
  (:Pressed
    (Rendering|Components|TextRender|SetXScale _press_e 1.2)
    (Rendering|Components|TextRender|SetYScale _press_e 1.2)
    (Utilities|FlowControl|Gate true
      (:Exit
        (Utilities|FlowControl|FlipFlop
          (:A
            (Components|Animation|PlayAnimation _skeletalmesh "/Game/ATACase/Anim_SK/Anim_ATACase_D_OpeningEx.Anim_ATACase_D_OpeningEx" false))
          (:B
            (Components|Animation|PlayAnimation _skeletalmesh "/Game/ATACase/Anim_SK/Anim_ATACase_D_Closing.Anim_ATACase_D_Closing" false))))))
  (:Released
    (Rendering|Components|TextRender|SetXScale _press_e 1.0)
    (Rendering|Components|TextRender|SetYScale _press_e 1.0)))

(fn ConstructionScript)