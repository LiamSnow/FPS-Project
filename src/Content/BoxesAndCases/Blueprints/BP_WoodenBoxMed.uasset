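; BP_WoodenBoxMed is a medium wooden box prop with a configurable lid angle and colors.
; The construction script sets the Cover's relative roll from RotationCover, then creates dynamic instances of MI_WoodenBoxMed for Cover and Hull.
; Both instances receive the COLOR, COLORScnd and Sighs vector parameters.
; CustomColor is reused for both, so it ends up holding only the Hull's instance.
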(fn ConstructionScript
  (Transformation|SetRelativeRotation (Variables|Default|GetCover) (Class|KismetMathLibrary|MakeRot 0.0 0.0 (Variables|Default|GetrotationCover)) false)
  (bind _returnvalue (Rendering|Material|CreateDynamicMaterialInstance (Variables|Default|GetCover) 0 "/Game/BoxesAndCases/Materials/MI_WoodenBoxMed.MI_WoodenBoxMed" :!class /Script/Engine.PrimitiveComponent))
  (bind _output_get (Variables|Default|SetCustomColor _returnvalue))
  (Rendering|Material|SetVectorParameterValue _output_get "customColor_param" (Variables|Default|GetCOLOR) :!class /Script/Engine.MaterialInstanceDynamic)
  (Rendering|Material|SetVectorParameterValue _returnvalue "customColor_param_b" (Variables|Default|GetCOLOR_scnd) :!class /Script/Engine.MaterialInstanceDynamic)
  (Rendering|Material|SetVectorParameterValue _returnvalue "customColor_param_c" (Variables|Default|GetSighs) :!class /Script/Engine.MaterialInstanceDynamic)
  (bind _returnvalue_2 (Rendering|Material|CreateDynamicMaterialInstance (Variables|Default|GetHull) 0 "/Game/BoxesAndCases/Materials/MI_WoodenBoxMed.MI_WoodenBoxMed" :!class /Script/Engine.PrimitiveComponent))
  (bind _output_get_2 (Variables|Default|SetCustomColor _returnvalue_2))
  (Rendering|Material|SetVectorParameterValue _output_get_2 "customColor_param" (Variables|Default|GetCOLOR) :!class /Script/Engine.MaterialInstanceDynamic)
  (Rendering|Material|SetVectorParameterValue _returnvalue_2 "customColor_param_b" (Variables|Default|GetCOLOR_scnd) :!class /Script/Engine.MaterialInstanceDynamic)
  (Rendering|Material|SetVectorParameterValue _returnvalue_2 "customColor_param_c" (Variables|Default|GetSighs) :!class /Script/Engine.MaterialInstanceDynamic))