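; BP_MetallCaseSmall is a small metal case prop with an adjustable cover angle and three customizable colors.
; Its construction script sets the cover's roll from RotationCover, then gives Cover and Hull separate dynamic instances of MI_MetallCaseSmall.
; Both instances receive the COLOR, DECALA and Sighs variables as color parameters.
; A RandomColor helper makes muted random colors, but the assignments that would use it are disconnected and never run.
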(fn ConstructionScript
  (Transformation|SetRelativeRotation (Variables|Default|GetCover) (Math|Rotator|MakeRotator (Variables|Default|GetrotationCover) 0.0 0.0) false false)
  (bind _returnvalue (Rendering|Material|CreateDynamicMaterialInstance (Variables|Default|GetCover) 0 "/Game/BoxesAndCases/Materials/MI_MetallCaseSmall.MI_MetallCaseSmall" :!class /Script/Engine.PrimitiveComponent))
  (bind _output_get (Variables|Default|SetCustomColor _returnvalue))
  (Rendering|Material|SetVectorParameterValue _output_get "customColor_param" (Variables|Default|GetCOLOR) :!class /Script/Engine.MaterialInstanceDynamic)
  (Rendering|Material|SetVectorParameterValue _returnvalue "customColor_param_b" (Variables|Default|GetDECAL_a) :!class /Script/Engine.MaterialInstanceDynamic)
  (Rendering|Material|SetVectorParameterValue _returnvalue "customColor_param_c" (Variables|Default|GetSighs) :!class /Script/Engine.MaterialInstanceDynamic)
  (bind _returnvalue_2 (Rendering|Material|CreateDynamicMaterialInstance (Variables|Default|GetHull) 0 "/Game/BoxesAndCases/Materials/MI_MetallCaseSmall.MI_MetallCaseSmall" :!class /Script/Engine.PrimitiveComponent))
  (bind _output_get_2 (Variables|Default|SetCustomColor _returnvalue_2))
  (Rendering|Material|SetVectorParameterValue _output_get_2 "customColor_param" (Variables|Default|GetCOLOR) :!class /Script/Engine.MaterialInstanceDynamic)
  (Rendering|Material|SetVectorParameterValue _returnvalue_2 "customColor_param_b" (Variables|Default|GetDECAL_a) :!class /Script/Engine.MaterialInstanceDynamic)
  (Rendering|Material|SetVectorParameterValue _returnvalue_2 "customColor_param_c" (Variables|Default|GetSighs) :!class /Script/Engine.MaterialInstanceDynamic))

(fn RandomColor
  (return (Utilities|Struct|MakeLinearColor (Math|Random|RandomFloatinRange 0.0 0.3) (Math|Random|RandomFloatinRange 0.0 0.5) (Math|Random|RandomFloatinRange 0.0 0.5) 1.0)))