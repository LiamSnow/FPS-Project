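; Main-menu loot crate that awards a random weapon skin from the game instance's skin list when MainMenuGuy fires its open-crate event.
; Opening shakes the crate via a delayed DoN loop feeding Tick's rotation interpolation, then timelines swing the lid and fly a spawned SprayCan to screen before showing the SkinRecieved widget.
; Dynamic materials drive tint, red hover glow and opacity fades; fading down also closes an open crate.
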(event Custom|CheckHovered
  (bind _asmain_menu_guy (Utilities|Casting|CastToMainMenuGuy (Game|GetPlayerCharacter 0)))
  (for _array_element (Variables|Default|GetDynamicSkins)
    (Rendering|Material|SetVectorParameterValue _array_element "Emissive" (select (Variables|/Game/Guns/Blueprints/MainMenuGuy.MainMenuGuy_C|GetHoveringOnCrate _asmain_menu_guy) "(R=10.000000,G=0.000000,B=0.000000,A=1.000000)" "") :!class /Script/Engine.MaterialInstanceDynamic)))

(event Custom|FadeUp
  (Variables|Default|SetEnabled true)
  (bind _newtrack_0 (Timeline|Timeline_2 Play)
    (:Update
      (for _array_element (Variables|Default|GetDynamicSkins)
        (Rendering|Material|SetScalarParameterValue _array_element "Opacity" _newtrack_0 :!class /Script/Engine.MaterialInstanceDynamic)))))

(event Custom|FadeDown
  (Variables|Default|SetEnabled false)
  (Utilities|FlowControl|Sequence
    (:then_0
      (bind _newtrack_0 (Timeline|Timeline_2 Reverse)
        (:Update
          (for _array_element (Variables|Default|GetDynamicSkins)
            (Rendering|Material|SetScalarParameterValue _array_element "Opacity" _newtrack_0 :!class /Script/Engine.MaterialInstanceDynamic)))))
    (:then_1
      (if (Variables|Default|GetOpen)
        (CallFunction|Hide)))))

(event Custom|OpenCrateEvent
  (bind _returnvalue (Math|Float|MakeLiteralFloat 0.08))
  (bind _returnvalue_2 (Class|KismetSystemLibrary|MakeLiteralInteger 20))
  (bind _self self)
  (bind _returnvalue_3 (Transformation|GetActorLocation _self))
  (bind _returnvalue_4 (+ _returnvalue_3 "0, 0,50.000000"))
  (bind _returnvalue_5 (Math|Transform|MakeTransform _returnvalue_4 "0, 0, 0" "0.000000,0.000000,0.000000"))
  (Variables|Default|SetEnabled false)
  (Variables|Default|SetOpen true)
  (Utilities|FlowControl|Sequence
    (:then_0
      (goto _label Reset))
    (:then_1
      (bind _counter (Utilities|FlowControl|DoN _returnvalue_2 :!label _label)
        (:Exit
          (Variables|Default|SetMoveToRot (Math|Rotator|MakeRotator (Math|Random|RandomFloatinRange (Math|Float|MakeLiteralFloat (* -1 (* (Math|Conversions|ToFloat(Integer) _counter) 0.7))) (Math|Float|MakeLiteralFloat (* (Math|Conversions|ToFloat(Integer) _counter) 0.7))) (Math|Random|RandomFloatinRange (Math|Float|MakeLiteralFloat (* -1 (* (Math|Conversions|ToFloat(Integer) _counter) 0.7))) (Math|Float|MakeLiteralFloat (* (Math|Conversions|ToFloat(Integer) _counter) 0.7))) (- (Math|Random|RandomFloatinRange (Math|Float|MakeLiteralFloat (* -1 (* (Math|Conversions|ToFloat(Integer) _counter) 0.7))) (Math|Float|MakeLiteralFloat (* (Math|Conversions|ToFloat(Integer) _counter) 0.7))) 7e+01)))
          (Utilities|FlowControl|Delay _returnvalue)
          (goto _label))))
    (:then_2
      (Utilities|FlowControl|Delay (* _returnvalue_2 _returnvalue))
      (Utilities|FlowControl|Sequence
        (:then_0
          (bind _newtrack_0 (Timeline|OpenCrate PlayFromStart)
            (:Update
              (Variables|Default|SetrotationCover (* _newtrack_0 -9e+01)))))
        (:then_1
          (bind _asthe_game_instance (Utilities|Casting|CastToTheGameInstance (Game|GetGameInstance)))
          (Variables|Default|SetRandSkin (Utilities|Array|Get(acopy) (Variables|/Game/Guns/Maps/TheGameInstance.TheGameInstance_C|GetAllSkins _asthe_game_instance) (Math|Random|RandomIntegerinRange 0 (Utilities|Array|Length (Variables|/Game/Guns/Maps/TheGameInstance.TheGameInstance_C|GetAllSkins _asthe_game_instance)))))
          (Utilities|FlowControl|Delay 0.5)
          (bind _returnvalue_6 (Game|SpawnActorfromClass "/Game/BoxesAndCases/Blueprints/SprayCan.SprayCan_C" _returnvalue_5 "AlwaysSpawn" 0 (Variables|Default|GetRandSkin) 0))
          (Variables|Default|SetSprayCan _returnvalue_6)
          (Variables|Default|SetSprayCanStartLocation _returnvalue_5)
          (bind _asmain_menu_guy (Utilities|Casting|CastToMainMenuGuy (Game|GetPlayerCharacter 0)))
          (Variables|Default|SetSprayCanTargetLocation (Transformation|GetWorldTransform (Variables|/Game/Guns/Blueprints/MainMenuGuy.MainMenuGuy_C|GetSprayCanPos _asmain_menu_guy)))
          (bind _newtrack_1 (Timeline|MoveToScreen PlayFromStart)
            (:Update
              (Transformation|SetActorScale3D (Variables|Default|GetSprayCan) (Math|Vector|MakeVector _newtrack_1 _newtrack_1 _newtrack_1))
              (Transformation|SetActorLocation (Variables|Default|GetSprayCan) (Math|Vector|Lerp(Vector) (.Location (Math|Transform|BreakTransform (Variables|Default|GetSprayCanStartLocation))) (.Location (Math|Transform|BreakTransform (Variables|Default|GetSprayCanTargetLocation))) _newtrack_1) false false)
              (Transformation|SetActorRotation (Variables|Default|GetSprayCan) (Math|Rotator|Lerp(Rotator) (.Rotation (Math|Transform|BreakTransform (Variables|Default|GetSprayCanStartLocation))) (.Rotation (Math|Transform|BreakTransform (Variables|Default|GetSprayCanTargetLocation))) _newtrack_1)))
            (:Finished
              (bind _returnvalue_7 (UserInterface|CreateWidget "/Game/Hud/Widgets/Common/SkinRecieved.SkinRecieved_C" 0 self (Variables|Default|GetRandSkin)))
              (UserInterface|Viewport|AddtoViewport _returnvalue_7 5))))))))

(event Custom|Hide
  (Utilities|FlowControl|Sequence
    (:then_0
      (bind _newtrack_0 (Timeline|Timeline_1 ReverseFromEnd)
        (:Update
          (Transformation|SetActorScale3D (Variables|Default|GetSprayCan) (Math|Vector|MakeVector _newtrack_0 _newtrack_0 _newtrack_0)))))
    (:then_1
      (Utilities|FlowControl|Delay 0.5)
      (bind _newtrack_0_2 (Timeline|Timeline_0 ReverseFromEnd)
        (:Update
          (Variables|Default|SetrotationCover (* _newtrack_0_2 -9e+01)))))
    (:then_2
      (Utilities|FlowControl|Delay 0.65)
      (Variables|Default|SetMoveToRot "0,-70.000000, 0"))
    (:then_3
      (Variables|Default|SetEnabled true)
      (Variables|Default|SetOpen false))))

(event EventBeginPlay
  (Utilities|Time|SetTimerbyEvent (delegate Custom|CheckHovered) 0.1 true)
  (bind _asmain_menu_guy (Utilities|Casting|CastToMainMenuGuy (Game|GetPlayerCharacter 0)))
  (EventDispatchers|BindEventtoOpenCrate _asmain_menu_guy (delegate Custom|OpenCrateEvent)))

(event EventTick
  (params (DeltaSeconds :type Float%20%28single-precision%29))
  (Transformation|SetRelativeRotation (Variables|Default|GetCover) (Math|Rotator|MakeRotator (Variables|Default|GetrotationCover) 0.0 0.0) false false)
  (Transformation|SetActorRotation (Math|Interpolation|RInterpTo (Transformation|GetActorRotation) (Variables|Default|GetMoveToRot) DeltaSeconds 11.0)))

(fn ConstructionScript
  (Transformation|SetRelativeRotation (Variables|Default|GetCover) (Math|Rotator|MakeRotator (Variables|Default|GetrotationCover) 0.0 0.0) false false)
  (bind _returnvalue (Rendering|Material|CreateDynamicMaterialInstance (Variables|Default|GetCover) 0 "/Game/BoxesAndCases/Materials/MI_MetallCaseSmall.MI_MetallCaseSmall" :!class /Script/Engine.PrimitiveComponent))
  (Utilities|Array|Add (Variables|Default|GetDynamicSkins) _returnvalue)
  (bind _output_get (Variables|Default|SetCustomColor _returnvalue))
  (Rendering|Material|SetVectorParameterValue _output_get "customColor_param" (Variables|Default|GetCOLOR) :!class /Script/Engine.MaterialInstanceDynamic)
  (Rendering|Material|SetVectorParameterValue _returnvalue "customColor_param_b" (Variables|Default|GetDECAL_a) :!class /Script/Engine.MaterialInstanceDynamic)
  (Rendering|Material|SetVectorParameterValue _returnvalue "customColor_param_c" (Variables|Default|GetSighs) :!class /Script/Engine.MaterialInstanceDynamic)
  (bind _returnvalue_2 (Rendering|Material|CreateDynamicMaterialInstance (Variables|Default|GetHull) 0 "/Game/BoxesAndCases/Materials/MI_MetallCaseSmall.MI_MetallCaseSmall" :!class /Script/Engine.PrimitiveComponent))
  (Utilities|Array|Add (Variables|Default|GetDynamicSkins) _returnvalue_2)
  (bind _output_get_2 (Variables|Default|SetCustomColor _returnvalue_2))
  (Rendering|Material|SetVectorParameterValue _output_get_2 "customColor_param" (Variables|Default|GetCOLOR) :!class /Script/Engine.MaterialInstanceDynamic)
  (Rendering|Material|SetVectorParameterValue _returnvalue_2 "customColor_param_b" (Variables|Default|GetDECAL_a) :!class /Script/Engine.MaterialInstanceDynamic)
  (Rendering|Material|SetVectorParameterValue _returnvalue_2 "customColor_param_c" (Variables|Default|GetSighs) :!class /Script/Engine.MaterialInstanceDynamic)
  (for _array_element (Variables|Default|GetDynamicSkins)
    (Rendering|Material|SetScalarParameterValue _array_element "Opacity" 0.0 :!class /Script/Engine.MaterialInstanceDynamic)))

(fn RandomColor
  (return (Utilities|Struct|MakeLinearColor (Math|Random|RandomFloatinRange 0.0 0.3) (Math|Random|RandomFloatinRange 0.0 0.5) (Math|Random|RandomFloatinRange 0.0 0.5) 1.0)))